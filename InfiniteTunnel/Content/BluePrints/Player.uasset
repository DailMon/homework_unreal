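; Player pawn for an endless-runner style tunnel flyer, moving forward at ever-increasing speed while axis input strafes it.
; BeginPlay creates the HUD and chains five tunnels via SpawnPoint, placing random obstacles at the joins.
; Overlaps go through CastToObstacle, which also applies effects: bombs reload the level, boosts add speed, slows temporarily halve strafing.
; Coins update the HUD counter and exponentially shrink the material's TextureGreen parameter.
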(event `self.ReceiveBeginPlay`
  (bind _returnvalue (`|GenericCreateObject` "/Game/BluePrints/MyHUD.MyHUD_C" self))
  (bind _output_get (set `self.HUDInstance` _returnvalue))
  (`UserWidget.AddToViewport` _output_get 0)
  (`self.SetCollectedText` 0)
  (bind _returnvalue_2 (`PrimitiveComponent.CreateDynamicMaterialInstance` (`self.PlayerRoot`) 0 null "None"))
  (set `self.OurMaterial` _returnvalue_2)
  (for _ (range 5)
    (`/Engine/EditorBlueprintResources/StandardMacros.IsValid` (`self.LastSpawnedTunnel`)
      (:`Is Valid`
        (`self.SpawnNextTunnel`))
      (:`Is Not Valid`
        (`self.SpawnTunnel` (0.0 0.0 0.0))))))

(event `self.ReceiveActorBeginOverlap`
  (params (OtherActor :type "Actor Object Reference"))
  (bind _numberobstacle (`self.CastToObstacle` OtherActor))
  (switch `int` _numberobstacle
    (:`0`
      (`GameplayStatics.OpenLevel` "Game_level"))
    (:`1`
      (`self.K2_DestroyActor` OtherActor))
    (:`2`
      (`self.K2_DestroyActor` OtherActor)
      (`KismetSystemLibrary.Delay` 3.0)
      (set `self.StrafeSpeed` (* (`self.StrafeSpeed`) 2.0)))))

(event `self.ReceiveTick`
  (params (DeltaSeconds :type "Float (single-precision)"))
  (bind _returnvalue (`self.ConsumeMovementInputVector`))
  (`SceneComponent.K2_AddLocalOffset` (`self.PlayerRoot`) (+ (* _returnvalue (* DeltaSeconds (`self.StrafeSpeed`))) (* (`self.GetActorForwardVector`) (* (`self.FlightSpeed`) DeltaSeconds))) true false)
  (set `self.FlightSpeed` (+ (`self.FlightSpeed`) (* (`self.FlightAcceleration`) DeltaSeconds))))

(event `InputAxis|AxisX`
  (params (AxisValue :type "Float (single-precision)"))
  (`self.AddMovementInput` (`KismetMathLibrary.GetRightVector` (struct)) AxisValue))

(event `InputAxis|AxisY`
  (params (AxisValue :type "Float (single-precision)"))
  (`self.AddMovementInput` (`KismetMathLibrary.GetUpVector` (struct)) AxisValue))

(fn `CastToObstacle`
  (params (Object :type "Actor Object Reference"))
  (returns (NumberObstacle :type Integer))
  (locals (NewLocalVar_0 :type "Float (double-precision)" :default 0.0))
  (cast `/Game/BluePrints/Bomb` Object
    (:`then`
      (return 0))
    (:`CastFailed`
      (cast `/Game/BluePrints/Boost` Object
        (:`then`
          (set `self.FlightSpeed` (+ (`self.FlightSpeed`) 150.0)))
        (:`CastFailed`
          (cast `/Game/BluePrints/Slow` Object
            (:`then`
              (set `self.StrafeSpeed` (/ (`self.StrafeSpeed`) 2.0))
              (return 2))
            (:`CastFailed`
              (cast `/Game/BluePrints/Coin` Object
                (:`then`
                  (bind _result (`/Engine/EditorBlueprintResources/StandardMacros.IncrementInt` (`self.CollectedCoins`))
                    (:`  `
                      (bind _output_get (set `self.CollectedCoins` _result))
                      (`self.SetCollectedText` _output_get)
                      (`MaterialInstanceDynamic.SetScalarParameterValue` (`self.OurMaterial`) "TextureGreen" (/ 1.0 (`KismetMathLibrary.MultiplyMultiply_FloatFloat` 10.0 (`KismetMathLibrary.Conv_IntToDouble` _output_get)))))))
                (:`CastFailed`
                  (return 3)))))))
      (return 1))))

(fn `SetCollectedText`
  (params (Collected :type Integer))
  (`TextBlock.SetText` (`/Game/BluePrints/MyHUD.TextCollectedCoins` (`self.HUDInstance`)) (`|FormatText` "Collected Coins: {Collected}" Collected)))

(fn `SpawnNextTunnel`
  (bind _returnvalue (`SceneComponent.K2_GetComponentLocation` (`/Game/BluePrints/Tunnel.SpawnPoint` (`self.LastSpawnedTunnel`))))
  (`self.SpawnTunnel` _returnvalue)
  (`self.SpawnRandomObstacle` _returnvalue))

(fn `SpawnRandomObstacle`
  (params (Location :type "Vector Structure"))
  (bind _returnvalue (`KismetMathLibrary.MakeVector` 0.2 0.2 0.2))
  (bind _returnvalue_2 (`KismetMathLibrary.Conv_VectorToRotator` (`KismetMathLibrary.MakeVector` 0.0 0.0 90.0)))
  (bind _returnvalue_3 (+ Location (`KismetMathLibrary.MakeVector` 0.0 (`KismetMathLibrary.RandomFloatInRange` -40.0 40.0) (`KismetMathLibrary.RandomFloatInRange` -40.0 40.0))))
  (switch `int` (`KismetMathLibrary.RandomInteger` 4)
    (:`0`
      (`|SpawnActorFromClass` "/Game/BluePrints/Boost.Boost_C" (`KismetMathLibrary.MakeTransform` _returnvalue_3 _returnvalue_2 _returnvalue) "Undefined" "OverrideRootScale" null null))
    (:`1`
      (`|SpawnActorFromClass` "/Game/BluePrints/Slow.Slow_C" (`KismetMathLibrary.MakeTransform` _returnvalue_3 _returnvalue_2 _returnvalue) "Undefined" "OverrideRootScale" null null))
    (:`2`
      (`|SpawnActorFromClass` "/Game/BluePrints/Bomb.Bomb_C" (`KismetMathLibrary.MakeTransform` _returnvalue_3 (struct) _returnvalue) "Undefined" "OverrideRootScale" null null))
    (:`3`
      (`|SpawnActorFromClass` "/Game/BluePrints/Coin.Coin_C" (`KismetMathLibrary.MakeTransform` _returnvalue_3 (struct) _returnvalue) "Undefined" "OverrideRootScale" null null))))

(fn `SpawnTunnel`
  (params (Location :type "Vector Structure"))
  (bind _returnvalue (`|SpawnActorFromClass` "/Game/BluePrints/Tunnel.Tunnel_C" (`KismetMathLibrary.MakeTransform` Location) "Undefined" "OverrideRootScale" null null))
  (set `self.LastSpawnedTunnel` _returnvalue))

(fn `UserConstructionScript`)